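; Dialogue component for the Bananafish Ben NPC, running its branching conversation about missing glasses.
; BeginPlay caches the owning PC_BANANAFISH_BEN_CHILD, and the Dialogue override picks a tree by DialogueTreeIndex, chaining AddDialogue calls that branch on the chosen option.
; Endings reset, rewind or clear progress before closing the conversation, and refusing to help also swaps Ben's sprite flipbook, flagged in a comment as problematic.
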(event `self.ReceiveBeginPlay`
  (bind _aspc_bananafish_ben_child (cast `/Game/Game_Systems/Paper2DSystem/PC_BANANAFISH_BEN_CHILD` (`self.GetOwner`)))
  (set `self.angrybananafishitself` _aspc_bananafish_ben_child))

(fn `Dialogue`
  (locals (NewLocalVar :type Text :default "NSLOCTEXT(\"[F52B57F972E5159588D04A7F7072A5A1]\", \"D2CB5229474778DDEBD7CB94B6C2C76E\", \"No\")"))
  (`parent.Dialogue`)
  (switch `int` (`self.DialogueTreeIndex`)
    (:`0`
      (bind (_state _newparam) (`self.AddDialogue` "angryBananaFish" "Did you see my glasses?" (`|MakeArray` "Yes" "No" :!type "Text") "/Game/Audio/Test/WhatsApp_Audio_2026-09-08_at_10_40_51_01.WhatsApp_Audio_2026-09-08_at_10_40_51_01"))
      (switch `/Game/Game_Systems/DialogueSystem/Enum_DialogueState` _state
        (:`NewEnumerator0`
          (switch `int` _newparam
            (:`0`
              (bind (_state_2 _newparam_2) (`self.AddDialogue` "angryBananaFish" "Can you pass it to me?" (`|MakeArray` "Yes" "No" :!type "Text") "/Game/Audio/Test/WhatsApp_Audio_2026-09-08_at_10_40_51_01.WhatsApp_Audio_2026-09-08_at_10_40_51_01"))
              (switch `/Game/Game_Systems/DialogueSystem/Enum_DialogueState` _state_2
                (:`NewEnumerator0`
                  (switch `int` _newparam_2
                    (:`0`
                      (bind _state_3 (`self.AddDialogue` "" "thanks" (`|MakeArray` "Continue" :!type "Text") "/Game/Audio/Test/WhatsApp_Audio_2026-09-08_at_10_40_51_01.WhatsApp_Audio_2026-09-08_at_10_40_51_01"))
                      (switch `/Game/Game_Systems/DialogueSystem/Enum_DialogueState` _state_3
                        (:`NewEnumerator0`
                          (`self.SetDialogueTreeIndex` 0)
                          (`self.CloseConversation`))))
                    (:`1`
                      (bind _state_4 (`self.AddDialogue` "" "nahhhh" (`|MakeArray` "Continue" :!type "Text") "/Game/Audio/Test/WhatsApp_Audio_2026-09-08_at_10_40_51_01.WhatsApp_Audio_2026-09-08_at_10_40_51_01"))
                      (switch `/Game/Game_Systems/DialogueSystem/Enum_DialogueState` _state_4
                        (:`NewEnumerator0`
                          (`self.RemoveDialogueProgression` 2)
                          (`self.CloseConversation`))))))))
            (:`1`
              (bind _state_5 (`self.AddDialogue` "angryBananaFish" "But I need it!" (`|MakeArray` "Continue" :!type "Text") "/Game/Audio/Test/WhatsApp_Audio_2026-09-08_at_10_40_51_01.WhatsApp_Audio_2026-09-08_at_10_40_51_01"))
              ; problem of changing child character sprite flipbook
              (switch `/Game/Game_Systems/DialogueSystem/Enum_DialogueState` _state_5
                (:`NewEnumerator0`
                  (`PaperFlipbookComponent.SetFlipbook` (`PaperCharacter.Sprite` (`self.angrybananafishitself`)) "/Game/Game_Systems/Paper2DSystem/FB_BENIDLETEST.FB_BENIDLETEST")
                  (`self.ClearDialogueProgress`)
                  (`self.CloseConversation`))))))))
    (:`1`
      (bind _state_6 (`self.AddDialogue` "angryBananaFish" "yipee" (`|MakeArray` "Continue" :!type "Text") "/Game/Audio/Test/WhatsApp_Audio_2026-09-08_at_10_40_51_01.WhatsApp_Audio_2026-09-08_at_10_40_51_01"))
      (switch `/Game/Game_Systems/DialogueSystem/Enum_DialogueState` _state_6
        (:`NewEnumerator0`
          (`self.ClearDialogueProgress`)
          (`self.CloseConversation`))))))