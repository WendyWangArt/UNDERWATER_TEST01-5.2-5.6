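; PC_BANANAFISH_BEN is a Paper2D interactable character, apparently a banana fish NPC, with a flipbook sprite and a name label.
; Construction writes CharacterName into the label, and BeginPlay sets the sprite to the FishIdle flipbook.
; SetInteractableState shows or hides the label, and ConversationClosed forwards a conversation-closed message to the interacting instigator.
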(event `self.ReceiveBeginPlay`
  (`PaperFlipbookComponent.SetFlipbook` (`self.Sprite`) (`self.fishIdle`)))

(event `/Game/Game_Systems/DialogueSystem/BluePrint_Interactable.SetInteractableState`
  (params (`CanShowInteract?` :type Boolean))
  (if `CanShowInteract?`
    (`SceneComponent.SetVisibility` (`self.txtCharacterName`) true false)
    (else
      (`SceneComponent.SetVisibility` (`self.txtCharacterName`) false false))))

(event `/Game/Game_Systems/DialogueSystem/BluePrint_Interactable.ConversationClosed`
  (message `/Game/Game_Systems/DialogueSystem/BluePrint_Interactable.ConversationClosed` (`self.InteractingInstigator`)))

(fn `UserConstructionScript`
  (`TextRenderComponent.K2_SetText` (`self.txtCharacterName`) (`self.CharacterName`)))